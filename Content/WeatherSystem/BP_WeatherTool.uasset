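; BP_WeatherTool is a weather actor that raises or lowers rain intensity and its effects on surfaces and clouds.
; IncreaseWeather and DecreaseWeather step a shared Value that drives MF_WeatherCollection material parameters, Rain spawn rate, volumetric cloud layers and splash frequency.
; From BeginPlay, SplashTest runs a Delay-paced loop of randomized downward line traces around the actor, spawning splash or ripple emitters at hits while rain is enabled, with optional debug drawing.
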(event Custom|SplashTest
  (bind _self self)
  (bind _area_of_splash_ (Variables|Default|GetArea%20of%20Splash%20))
  (bind _returnvalue (Transformation|GetActorLocation _self))
  (bind _returnvalue_2 (* _area_of_splash_ -1.0))
  (bind _returnvalue_3 (Math|Random|RandomFloatinRange _returnvalue_2 _area_of_splash_))
  (bind _returnvalue_4 (Math|Random|RandomFloatinRange _returnvalue_2 _area_of_splash_))
  (bind (_x _y _z) (Math|Vector|BreakVector _returnvalue))
  (bind _returnvalue_5 (+ _y _returnvalue_4))
  (bind _returnvalue_6 (+ _x _returnvalue_3))
  ;[1 1 1] Splash FX Loop
  (for _index (range 1 (Variables|Default|GetMutiple%20of%20Splash)) :!label _label
    (if (Variables|Default|GetEnable%20Rain%20System)
      (bind (_outhit _returnvalue_7) (Collision|LineTraceByChannel (Math|Vector|MakeVector _returnvalue_6 _returnvalue_5 (+ _z 2e+03)) (Math|Vector|MakeVector _returnvalue_6 _returnvalue_5 (+ _z -1e+03)) "TraceTypeQuery1" (Variables|Default|GetEnable%20Splash%20Hit%20TraceComplex) 0 "None" true "(R=1.000000,G=0.000000,B=0.000000,A=1.000000)" "(R=0.000000,G=1.000000,B=0.000000,A=1.000000)" 1.0))
      (if _returnvalue_7
        (if (Variables|Default|GetEnable%20Debug%20Mode)
          (Rendering|Debug|DrawDebugLine (.TraceStart (Collision|BreakHitResult _outhit)) (.TraceEnd (Collision|BreakHitResult _outhit)) "(R=1.000000,G=0.000000,B=0.000000,A=1.000000)" 0.1 2.0)
          (Rendering|Debug|DrawDebugSphere (.Location (Collision|BreakHitResult _outhit)) 12.0 12 "(R=1.000000,G=0.000000,B=0.000000,A=1.000000)" 0.1 2.0))
        (if (Variables|Default|GetEnable%20Splash%20With%20Ripple)
          (Effects|SpawnEmitteratLocation "/Game/WeatherSystem/Particles/PS_Splash_Ripple.PS_Splash_Ripple" (.Location (Collision|BreakHitResult _outhit)) "0, 0, 0" "0.500000,0.500000,0.500000")
          (else
            (Effects|SpawnEmitteratLocation "/Game/WeatherSystem/Particles/PS_Splash.PS_Splash" (.Location (Collision|BreakHitResult _outhit)) "0, 0, 0" "0.500000,0.500000,0.500000"))))
      (Utilities|FlowControl|Delay (/ 1.0 (* (Variables|Default|GetAmount%20of%20Rain) (Variables|Default|GetFrequency%20of%20Splash%20))))
      (goto _label)))
  (Utilities|FlowControl|Delay (/ 1.0 (* (Variables|Default|GetAmount%20of%20Rain) (Variables|Default|GetFrequency%20of%20Splash%20))))
  (goto _label))

(event Custom|Increase%20Weather
  (bind _output_get (Variables|Default|Setvalue (+ (Variables|Default|Getvalue) 0.02)))
  (if (> _output_get 0.0)
    (Variables|Default|SetEnable%20Rain%20System true))
  (Rendering|Material|SetScalarParameterValue "/Game/WeatherSystem/MatCollection/MF_WeatherCollection.MF_WeatherCollection" "Puddle Param" (Math|Float|Clamp(Float) (+ (Variables|Default|Getvalue) 0.02)) :!class /Script/Engine.KismetMaterialLibrary)
  (Rendering|Material|SetScalarParameterValue "/Game/WeatherSystem/MatCollection/MF_WeatherCollection.MF_WeatherCollection" "Rain Value" (Math|Float|Clamp(Float) (+ (Variables|Default|Getvalue) 0.02)) :!class /Script/Engine.KismetMaterialLibrary)
  (Rendering|Material|SetScalarParameterValue "/Game/WeatherSystem/MatCollection/MF_WeatherCollection.MF_WeatherCollection" "Roughness" (Math|Float|Clamp(Float) (+ (Variables|Default|Getvalue) 0.02)) :!class /Script/Engine.KismetMaterialLibrary)
  (Rendering|Material|SetScalarParameterValue "/Game/WeatherSystem/MatCollection/MF_WeatherCollection.MF_WeatherCollection" "Wind Param" (Math|Float|Clamp(Float) (+ (Variables|Default|Getvalue) 0.02)) :!class /Script/Engine.KismetMaterialLibrary)
  (Rendering|Material|SetScalarParameterValue "/Game/WeatherSystem/MatCollection/MF_WeatherCollection.MF_WeatherCollection" "Normal Param" 1.0 :!class /Script/Engine.KismetMaterialLibrary)
  (Rendering|Material|SetScalarParameterValue "/Game/WeatherSystem/MatCollection/MF_WeatherCollection.MF_WeatherCollection" "Roughness" (Math|Float|Clamp(Float) (+ (Variables|Default|Getvalue) 0.02)) :!class /Script/Engine.KismetMaterialLibrary)
  (Rendering|Material|SetScalarParameterValue "/Game/WeatherSystem/MatCollection/MF_WeatherCollection.MF_WeatherCollection" "Wetness Param" (Math|Float|Clamp(Float) (+ (Variables|Default|Getvalue) 0.02)) :!class /Script/Engine.KismetMaterialLibrary)
  (Rendering|Material|SetScalarParameterValue "/Game/WeatherSystem/MatCollection/MF_WeatherCollection.MF_WeatherCollection" "Metallic Value" 0.8 :!class /Script/Engine.KismetMaterialLibrary)
  (Effects|Components|ParticleSystem|SetFloatParameter (Variables|Default|GetRain) "SpawnRate" (Math|Float|Clamp(Float) (* (Math|Float|Clamp(Float) (+ (Variables|Default|Getvalue) 0.02)) 1e+01)))
  ;[1 1 1] Clouds
  (Class|VolumetricCloudComponent|SetLayerBottomAltitude (Variables|/Script/Engine.VolumetricCloud|GetVolumetricCloudComponent (Variables|Default|GetVolumetricCloud)) (Math|Float|Clamp(Float) (* (Variables|Default|Getvalue) -1e+01) 0.0 5.0))
  (Class|VolumetricCloudComponent|SetLayerHeight (Variables|/Script/Engine.VolumetricCloud|GetVolumetricCloudComponent (Variables|Default|GetVolumetricCloud)) (Math|Float|Clamp(Float) (* (Variables|Default|Getvalue) -5e+01) 1e+01 2e+01))
  ;[1 1 1] SplashFRQ
  (Variables|Default|SetFrequency%20of%20Splash%20 (Math|Float|Clamp(Float) (* (Variables|Default|Getvalue) 2e+01) 0.0 1.2e+02)))

(event Custom|Decrease%20Weather
  (bind _output_get (Variables|Default|Setvalue (- (Variables|Default|Getvalue) 0.05)))
  (if (>= _output_get 0.2)
    (Variables|Default|SetEnable%20Rain%20System false))
  (Rendering|Material|SetScalarParameterValue "/Game/WeatherSystem/MatCollection/MF_WeatherCollection.MF_WeatherCollection" "Puddle Param" (Math|Float|Clamp(Float) _output_get) :!class /Script/Engine.KismetMaterialLibrary)
  (Rendering|Material|SetScalarParameterValue "/Game/WeatherSystem/MatCollection/MF_WeatherCollection.MF_WeatherCollection" "Rain Value" (Math|Float|Clamp(Float) _output_get) :!class /Script/Engine.KismetMaterialLibrary)
  (Rendering|Material|SetScalarParameterValue "/Game/WeatherSystem/MatCollection/MF_WeatherCollection.MF_WeatherCollection" "Roughness" (Math|Float|Clamp(Float) _output_get) :!class /Script/Engine.KismetMaterialLibrary)
  (Rendering|Material|SetScalarParameterValue "/Game/WeatherSystem/MatCollection/MF_WeatherCollection.MF_WeatherCollection" "Wind Param" (Math|Float|Clamp(Float) _output_get) :!class /Script/Engine.KismetMaterialLibrary)
  (Rendering|Material|SetScalarParameterValue "/Game/WeatherSystem/MatCollection/MF_WeatherCollection.MF_WeatherCollection" "Roughness" (Math|Float|Clamp(Float) _output_get) :!class /Script/Engine.KismetMaterialLibrary)
  (Rendering|Material|SetScalarParameterValue "/Game/WeatherSystem/MatCollection/MF_WeatherCollection.MF_WeatherCollection" "Wetness Param" (Math|Float|Clamp(Float) _output_get) :!class /Script/Engine.KismetMaterialLibrary)
  (Rendering|Material|SetScalarParameterValue "/Game/WeatherSystem/MatCollection/MF_WeatherCollection.MF_WeatherCollection" "Normal Param" 0.1 :!class /Script/Engine.KismetMaterialLibrary)
  (Rendering|Material|SetScalarParameterValue "/Game/WeatherSystem/MatCollection/MF_WeatherCollection.MF_WeatherCollection" "Metallic Value" 0.0 :!class /Script/Engine.KismetMaterialLibrary)
  (Effects|Components|ParticleSystem|SetFloatParameter (Variables|Default|GetRain) "SpawnRate" (Math|Float|Clamp(Float) _output_get))
  ;[1 1 1] Clouds
  (Class|VolumetricCloudComponent|SetLayerBottomAltitude (Variables|/Script/Engine.VolumetricCloud|GetVolumetricCloudComponent (Variables|Default|GetVolumetricCloud)) (Math|Float|Clamp(Float) (* (Variables|Default|Getvalue) -1e+01) 0.0 5.0))
  (Class|VolumetricCloudComponent|SetLayerHeight (Variables|/Script/Engine.VolumetricCloud|GetVolumetricCloudComponent (Variables|Default|GetVolumetricCloud)) (Math|Float|Clamp(Float) (* (Variables|Default|Getvalue) -5e+01) 1e+01 2e+01))
  (Effects|Components|ParticleSystem|SetFloatParameter (Variables|Default|GetRain) "SpawnRate" (Math|Float|Clamp(Float) (* (Variables|Default|Getvalue) 1e+01)))
  ;[1 1 1] SplashFRQ
  (Variables|Default|SetFrequency%20of%20Splash%20 (Math|Float|Clamp(Float) (* (Variables|Default|Getvalue) -2e+01) 0.0 1.2e+02)))

(event EventBeginPlay
  (bind _rain (Variables|Default|GetRain))
  (CallFunction|SplashTest)
  (Effects|Components|ParticleSystem|SetFloatParameter _rain "SpawnRate" 0.0)
  (Rendering|SetVisibility _rain true false))

(event Collision|EventActorBeginOverlap
  (params (OtherActor :type Actor%20Object%20Reference)))

(fn ConstructionScript)