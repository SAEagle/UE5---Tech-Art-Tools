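; Spline-driven construction tool that builds a string of light bulbs in the level, with optional point lights and hanging cables.
; The construction script places bulb meshes at fixed spacing, giving each a dynamic glass material and optional random roll.
; Socket positions, converted to actor space, anchor the lights and cable components linking neighboring bulbs.
; Colors are fixed or palette-random, with light and emissive colors rolled independently.
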(event EventBeginPlay)

(event EventTick
  (params (DeltaSeconds :type Float%20%28single-precision%29)))

(fn ConstructionScript
  (bind _spline (Variables|Default|GetSpline))
  (bind _arrayofbulbs (Variables|Default|GetArrayOfBulbs))
  (bind _miref (Variables|Default|GetMIRef))
  ;[1 1 1] Spawn Bulb Along Spline
  (Utilities|Array|Clear (Variables|Default|GetArrayOfBulbs))
  (for _index (range 0 (Math|Float|Floor (/ (Spline|GetSplineLength (Variables|Default|GetSpline)) (Variables|CableSetup|GetWireSectionLength))))
    (Variables|Default|SetCurrentIndex _index)
    (bind _returnvalue (AddComponent|AddStaticMeshComponent false (Math|Conversions|ToTransform(Vector) (Spline|GetLocationatDistanceAlongSpline _spline (* (Variables|CableSetup|GetWireSectionLength) (Variables|Default|GetCurrentIndex)) "Local"))))
    (Components|StaticMesh|SetStaticMesh _returnvalue (Variables|BulbSetup|GetPlacedBulb))
    (Rendering|SetCastShadow _returnvalue (Variables|BulbSetup|GetBulbCastShadow))
    (Transformation|SetRelativeRotation _returnvalue (Spline|GetRotationatDistanceAlongSpline _spline (* (Variables|CableSetup|GetWireSectionLength) (Variables|Default|GetCurrentIndex)) "Local") false false)
    (Utilities|Array|Add (Variables|Default|GetArrayOfBulbs) _returnvalue))
  ;[1 1 1] BulbSettings Setup
  (for _array_element (Variables|Default|GetArrayOfBulbs)
    (Variables|Default|SetBulbArrayElem _array_element)
    (Utilities|IsValid (Variables|Default|GetBulbArrayElem)
      (:Is%20Valid
        (CallFunction|BulbSetup (Variables|Default|GetBulbArrayElem))
        ;[1 1 1] EnableDisableLight
        (if (Variables|LightningSettings|GetIsLightEnabled?)
          ;[1 1 1] PointLightSetup
          (Utilities|IsValid (Variables|Default|GetBulbArrayElem)
            (:Is%20Valid
              (CallFunction|PointLightSetup (Math|Conversions|ToTransform(Vector) (Utilities|TransformfromRelativetoWorld (Variables|Default|GetBulbArrayElem) (Utilities|Array|Get(acopy) (Transformation|GetAllSocketNames (Variables|Default|GetBulbArrayElem)) (Variables|Default|GetSocketIndex)))))
              (CallFunction|LightColorRandomness)))
          (else
            ;[1 1 1] EmmisiveRandomnes
            (if (Variables|LightningSettings|GetRandomLightColors)
              ;[1 1 1] EmmisiveOnlyLeft
              (CallFunction|EmissiveRandomnes _miref)
              (else
                (Rendering|Material|SetVectorParameterValue _miref "Emissive Color" (Variables|LightningSettings|GetColor%20Value) :!class /Script/Engine.MaterialInstanceDynamic))))))))
  ;[1 1 1] Cables setups and settings
  (Utilities|Array|Clear (Variables|Default|GetArrayOfCables))
  (if (Variables|CableSetup|GetShowCable)
    (for (_array_element_2 _array_index) (Variables|Default|GetArrayOfBulbs)
      (Variables|Default|SetCurrentBulbMesh _array_element_2)
      (Variables|Default|SetCableCurrentIndex _array_index)
      (Utilities|IsValid (Utilities|Array|Get(acopy) _arrayofbulbs (Math|Integer|Clamp(Integer) (+ (Variables|Default|GetCableCurrentIndex) 1) 0 (- (Utilities|Array|Length _arrayofbulbs) 1)))
        (:Is%20Valid
          ;;[1 1 1] CablesSetup
          (CallFunction|CableSetup (Math|Conversions|ToTransform(Vector) (Utilities|TransformfromRelativetoWorld (Variables|Default|GetCurrentBulbMesh) "wire")) (Utilities|TransformfromRelativetoWorld (Utilities|Array|Get(acopy) _arrayofbulbs (Math|Integer|Clamp(Integer) (+ (Variables|Default|GetCableCurrentIndex) 1) 0 (- (Utilities|Array|Length _arrayofbulbs) 1))) "wire") (- (Utilities|TransformfromRelativetoWorld (Utilities|Array|Get(acopy) _arrayofbulbs (Math|Integer|Clamp(Integer) (+ (Variables|Default|GetCableCurrentIndex) 1) 0 (- (Utilities|Array|Length _arrayofbulbs) 1))) "wire") (Utilities|TransformfromRelativetoWorld (Variables|Default|GetCurrentBulbMesh) "wire"))))))))

(fn PointLightSetup
  (params (InTransform :type Transform%20%28by%20ref%29))
  (bind _returnvalue (AddComponent|AddPointLightComponent false InTransform))
  (Variables|Default|SetPointLightRef _returnvalue)
  (Rendering|Lighting|SetAttenuationRadius (Variables|Default|GetPointLightRef) (Variables|LightningSettings|GetPointLightAttenuationRadius))
  (Rendering|Components|Light|SetIntensity (Variables|Default|GetPointLightRef) (Variables|LightningSettings|GetPointLightIntensity)))

(fn BulbSetup
  (params (Target :type Primitive%20Component%20Object%20Reference))
  (bind _returnvalue (Transformation|GetWorldRotation Target))
  (bind _returnvalue_2 (Transformation|GetWorldRotation Target))
  (bind _returnvalue_3 (Rendering|Material|CreateDynamicMaterialInstance Target 1 "/Game/SplineTool/Materials/MI_Light_Bulb_Glass_Inst.MI_Light_Bulb_Glass_Inst" "None" :!class /Script/Engine.PrimitiveComponent))
  (Variables|Default|SetMIRef _returnvalue_3)
  (Rendering|Material|SetScalarParameterValue (Variables|Default|GetMIRef) "Emissive Strength" (Variables|LightningSettings|GetEmissive%20Strengh) :!class /Script/Engine.MaterialInstanceDynamic)
  (Rendering|Material|SetScalarParameterValue (Variables|Default|GetMIRef) "Refraction Min" (Variables|LightningSettings|GetRefraction%20Min) :!class /Script/Engine.MaterialInstanceDynamic)
  (Rendering|Material|SetScalarParameterValue (Variables|Default|GetMIRef) "Refraction Max" (Variables|LightningSettings|GetRefraction%20Max) :!class /Script/Engine.MaterialInstanceDynamic)
  (if (Variables|BulbSetup|GetIsRandomBulbRotationAllowed)
    ;[1 1 1] Quick randomes on the X
    (Transformation|SetWorldRotation Target (Math|Rotator|MakeRotator (+ (Math|Random|RandomFloatinRange (Variables|BulbSetup|GetBulbRandomMinRot) (Variables|BulbSetup|GetBulbRandomMaxRot)) 1.8e+02) (.pitch _returnvalue_2) (.yaw _returnvalue_2)) false false)
    (else
      (Transformation|SetWorldRotation Target (Math|Rotator|MakeRotator 1.8e+02 (.pitch _returnvalue) (.yaw _returnvalue)) false false))))

(fn CableSetup
  (params (RelativeTransform :type Transform) (CableEndLocation :type Vector) (CableLength :type Vector))
  (bind _returnvalue (AddComponent|AddCableComponent false RelativeTransform))
  (bind _output_get (Variables|Default|SetCableRef _returnvalue))
  (Variables|/Script/CableComponent.CableComponent|SetEndLocation _output_get CableEndLocation)
  (Variables|/Script/CableComponent.CableComponent|SetCableWidth (Variables|Default|GetCableRef) (Variables|CableSetup|GetCableWidgth))
  (Variables|/Script/CableComponent.CableComponent|SetbEnableStiffness (Variables|Default|GetCableRef) (Variables|CableSetup|GetCableStiffness))
  (Variables|/Script/CableComponent.CableComponent|SetSolverIterations (Variables|Default|GetCableRef) (Variables|CableSetup|GetSolverIterations))
  (Variables|/Script/CableComponent.CableComponent|SetCableLength (Variables|Default|GetCableRef) (Math|Vector|VectorLength CableLength))
  (Variables|/Script/CableComponent.CableComponent|SetCableGravityScale (Variables|Default|GetCableRef) (Variables|CableSetup|GetCable%20Gravity%20Scale))
  (Variables|/Script/CableComponent.CableComponent|SetCableForce (Variables|Default|GetCableRef) (Variables|CableSetup|GetCable%20Force))
  (Rendering|SetCastShadow (Variables|Default|GetCableRef) (Variables|CableSetup|GetCableSetCast%20Shadow))
  (Utilities|Array|Add (Variables|Default|GetArrayOfCables) (Variables|Default|GetCableRef)))

(fn EmissiveRandomnes
  (params (self2 :type Material%20Instance%20Dynamic%20Object%20Reference))
  (bind _randomcolorpallete (Variables|LightningSettings|GetRandomColorPallete))
  (Rendering|Material|SetVectorParameterValue self2 "Emissive Color" (Utilities|Array|Get(acopy) _randomcolorpallete (Math|Random|RandomIntegerinRange 0 (Utilities|Array|Length _randomcolorpallete))) :!class /Script/Engine.MaterialInstanceDynamic))

(fn LightColorRandomness
  (bind _randomcolorpallete (Variables|LightningSettings|GetRandomColorPallete))
  (bind _pointlightref (Variables|Default|GetPointLightRef))
  (bind _miref (Variables|Default|GetMIRef))
  (bind _returnvalue (Utilities|Array|Length _randomcolorpallete))
  (bind _returnvalue_2 (Math|Random|RandomIntegerinRange 0 _returnvalue))
  (bind _output (Utilities|Array|Get(acopy) _randomcolorpallete _returnvalue_2))
  (if (Variables|LightningSettings|GetRandomLightColors)
    (Rendering|Components|Light|SetLightColor _pointlightref _output true)
    (Rendering|Material|SetVectorParameterValue _miref "Emissive Color" _output :!class /Script/Engine.MaterialInstanceDynamic)
    (else
      (Rendering|Components|Light|SetLightColor _pointlightref (Variables|LightningSettings|GetColor%20Value) true)
      (Rendering|Material|SetVectorParameterValue _miref "Emissive Color" (Variables|LightningSettings|GetColor%20Value) :!class /Script/Engine.MaterialInstanceDynamic))))