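; BP_Spline_Wires is a utility pole actor that hangs two cables to the next pole in a chain.
; The Construction Script sets the pole mesh, offsets both wire connectors and ends each cable at the matching NextMesh connector in local space.
; Cable gravity is random or fixed per cable, with width applied only in the random branch.
; Without a valid NextMesh, the last pole destroys its cables.
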(event EventBeginPlay)

(event Collision|EventActorBeginOverlap
  (params (OtherActor :type Actor%20Object%20Reference)))

(event EventTick
  (params (DeltaSeconds :type Float%20%28single-precision%29)))

(fn ConstructionScript
  (bind _returnvalue (Math|Random|RandomFloatinRange 1.1 1.5))
  (bind _cable_width (Variables|Wire|GetCable%20Width))
  (bind _wirecable_1 (Variables|Default|GetWireCable_1))
  (bind _wirecable_2 (Variables|Default|GetWireCable_2))
  (bind _wireconnector_1 (Variables|Default|GetWireConnector_1))
  (bind _wireconnector_2 (Variables|Default|GetWireConnector_2))
  (bind _returnvalue_2 (Math|Conversions|ToFloat(Integer) _cable_width))
  (bind _returnvalue_3 (Transformation|GetWorldLocation _wireconnector_2))
  (bind _returnvalue_4 (Transformation|GetWorldLocation _wireconnector_1))
  (Components|StaticMesh|SetStaticMesh (Variables|Default|GetStaticMesh) (Variables|PoleMesh|GetMesh%20Pole))
  (if (Variables|Wire|GetReattachCables)
    _
    (else
      _))
  (Utilities|IsValid (Variables|Default|GetNextMesh)
    (:Is%20Valid
      ;[1 1 1] Connectors Offsets
      (Transformation|SetWorldLocation _wireconnector_1 (Math|Vector|MakeVector (+ (.x _returnvalue_4) (Variables|Wire|GetWC_1_OffsetX)) (+ (.y _returnvalue_4) (Variables|Wire|GetWC_1_OffsetY)) (+ (.z _returnvalue_4) (Variables|Wire|GetWC_1_OffsetZ))) false false)
      (Transformation|SetWorldLocation _wireconnector_2 (Math|Vector|MakeVector (+ (.x _returnvalue_3) (Variables|Wire|GetWC_2_OffsetX)) (+ (.y _returnvalue_3) (Variables|Wire|GetWC_2_OffsetY)) (+ (.z _returnvalue_3) (Variables|Wire|GetWC_2_OffsetZ))) false false)
      ;[1 1 1] Cable 1
      (Variables|/Script/CableComponent.CableComponent|SetEndLocation (Variables|Default|GetWireCable_1) (Math|Transform|InverseTransformLocation (Transformation|GetActorTransform) (Transformation|GetWorldLocation (Variables|BP_Spline_Wires_C|GetWireConnector_1 (Variables|Default|GetNextMesh)))))
      ;[1 1 1] Cable 2
      (Variables|/Script/CableComponent.CableComponent|SetEndLocation (Variables|Default|GetWireCable_2) (Math|Transform|InverseTransformLocation (Transformation|GetActorTransform) (Transformation|GetWorldLocation (Variables|BP_Spline_Wires_C|GetWireConnector_2 (Variables|Default|GetNextMesh)))))
      ;[1 1 1] Gravity & Cable Width
      (if (Variables|Wire|GetRandomGravity)
        (Variables|/Script/CableComponent.CableComponent|SetCableGravityScale _wirecable_1 _returnvalue)
        (Variables|/Script/CableComponent.CableComponent|SetCableWidth _wirecable_1 _returnvalue_2)
        (Variables|/Script/CableComponent.CableComponent|SetCableGravityScale _wirecable_2 _returnvalue)
        (Variables|/Script/CableComponent.CableComponent|SetCableWidth _wirecable_2 _returnvalue_2)
        (else
          (Variables|/Script/CableComponent.CableComponent|SetCableGravityScale (Variables|Default|GetWireCable_1) (Variables|Wire|GetCable_1_Gravity))
          (Variables|/Script/CableComponent.CableComponent|SetCableGravityScale (Variables|Default|GetWireCable_2) (Variables|Wire|GetCable_2_Gravity)))))
    (:Is%20Not%20Valid
      ;[1 1 1] Last Pole Destroy Cables
      (Components|DestroyComponent (Variables|Default|GetWireCable_1)))))