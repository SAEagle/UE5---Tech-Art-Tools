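; BP_Spline_Mesh is a construction-script spline tool that repeats a chosen static mesh along a spline as instanced static mesh instances.
; Spacing is the mesh's bounding-box X length plus an offset, and spline length divided by it sets the count.
; Each instance sits at its distance along the spline in local space with yaw from ZRot, as the look-at-next-point rotation is left unused.
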(event EventBeginPlay)

(event Collision|EventActorBeginOverlap
  (params (OtherActor :type Actor%20Object%20Reference)))

(event EventTick
  (params (DeltaSeconds :type Float%20%28single-precision%29)))

(fn ConstructionScript
  (bind _placedmesh (Variables|Default|GetPlacedMesh))
  (bind _returnvalue (StaticMesh|GetBoundingBox _placedmesh))
  (Components|StaticMesh|SetStaticMesh (Variables|Default|GetInstancedStaticMesh) (Variables|Default|GetPlacedMesh))
  (bind _output_get (Variables|Default|SetSpacing (+ (.X (Math|Vector|BreakVector (- (.max _returnvalue) (.min _returnvalue)))) (Variables|Default|GetOffset%20of%20Mesh))))
  (Variables|Default|SetNumberOf%20Instances (Math|Float|Truncate (/ (Spline|GetSplineLength (Variables|Default|GetSpline)) _output_get)))
  (for _index (range 0 (Math|Float|Truncate (/ (Spline|GetSplineLength (Variables|Default|GetSpline)) _output_get)))
    (Components|InstancedStaticMesh|AddInstance (Variables|Default|GetInstancedStaticMesh) (Math|Transform|MakeTransform (CallFunction|GetLocationatIndex _index) (Math|Rotator|MakeRotator 0.0 0.0 (Variables|Default|GetZ%20Rot))) false)))

(fn GetLocationatIndex
  (params (A :type Integer))
  (return (Spline|GetLocationatDistanceAlongSpline (Variables|Default|GetSpline) (* A (Variables|Default|GetSpacing)) "Local")))