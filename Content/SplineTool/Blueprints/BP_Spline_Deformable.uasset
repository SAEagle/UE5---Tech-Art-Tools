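; Spline tool actor that lays a chosen static mesh, such as a wire, along an editable spline as deformed segments.
; The construction script divides the spline length by a section length and adds one spline mesh component per section on a configurable forward axis.
; Each segment takes local start and end positions by distance along the spline, with tangents clamped to zero size to remove tangent noise.
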(event EventBeginPlay)

(event Collision|EventActorBeginOverlap
  (params (OtherActor :type Actor%20Object%20Reference)))

(event EventTick
  (params (DeltaSeconds :type Float%20%28single-precision%29)))

(fn ConstructionScript
  (for _index (range 0 (Math|Float|Truncate (/ (Spline|GetSplineLength (Variables|Default|GetSpline)) (Variables|MeshSetup|GetWireSectionLength))))
    (Variables|MeshSetup|SetIndexOfSplines _index)
    ;[1 1 1] Spline and Wire Setup
    (CallFunction|SplineMeshSetup)))

(fn GetLocationatIndex
  (params (A :type Integer))
  (return (Spline|GetLocationatDistanceAlongSpline (Variables|Default|GetSpline) (* A 0.0) "Local")))

(fn SplineMeshSetup
  (bind _indexofsplines (Variables|MeshSetup|GetIndexOfSplines))
  (bind _indexofsplines_2 (Variables|MeshSetup|GetIndexOfSplines))
  (bind _spline (Variables|Default|GetSpline))
  (bind _spline_2 (Variables|Default|GetSpline))
  (bind _wiresectionlength (Variables|MeshSetup|GetWireSectionLength))
  (bind _wiresectionlength_2 (Variables|MeshSetup|GetWireSectionLength))
  (bind _returnvalue (* _wiresectionlength_2 _indexofsplines_2))
  (bind _returnvalue_2 (+ _indexofsplines 1))
  (bind _returnvalue_3 (* _wiresectionlength _returnvalue_2))
  (bind _returnvalue_4 (AddComponent|AddSplineMeshComponent false))
  (SplineMesh|SetForwardAxis _returnvalue_4 (Variables|MeshSetup|GetForward%20Axis%20Of%20Mesh) true)
  (Components|StaticMesh|SetStaticMesh _returnvalue_4 (Variables|MeshSetup|GetPlacedSplineMesh))
  (SplineMesh|SetStartandEnd _returnvalue_4 (Spline|GetLocationatDistanceAlongSpline _spline_2 _returnvalue "Local") (Math|Vector|ClampVectorSize (Spline|GetTangentatDistanceAlongSpline _spline_2 _returnvalue "Local") 0.0 0.0) (Spline|GetLocationatDistanceAlongSpline _spline _returnvalue_3 "Local") (Math|Vector|ClampVectorSize (Spline|GetTangentatDistanceAlongSpline _spline _returnvalue_3 "Local") 0.0 0.0) true :!class /Script/Engine.SplineMeshComponent))