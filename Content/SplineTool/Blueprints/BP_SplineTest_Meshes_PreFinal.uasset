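; Spline-driven construction-script tool that builds a string of light bulbs and wire, previewed in the editor.
; Per wire-length step, it adds instanced bulbs spaced by mesh bounds plus offset, with optional point lights and a tinted emissive dynamic material.
; Wire uses spline mesh components with clamped tangents, but is skipped when bulbs and lights are both enabled.
; An instanced-wire path remains unconnected.
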(event EventBeginPlay)

(event Collision|EventActorBeginOverlap
  (params (OtherActor :type Actor%20Object%20Reference)))

(event EventTick
  (params (DeltaSeconds :type Float%20%28single-precision%29)))

(fn ConstructionScript
  (bind _placedbulb (Variables|Default|GetPlacedBulb))
  (bind _returnvalue (StaticMesh|GetBoundingBox _placedbulb))
  (Components|StaticMesh|SetStaticMesh (Variables|Default|GetInstancedBulb) (Variables|Default|GetPlacedBulb))
  (Variables|Default|SetSpacing (+ (.X (Math|Vector|BreakVector (- (.max _returnvalue) (.min _returnvalue)))) (Variables|Default|GetBulbOffset)))
  (for _index (range 0 (Math|Float|Truncate (/ (Spline|GetSplineLength (Variables|Default|GetSpline)) (Variables|Default|GetWireSectionLength))))
    (Variables|Default|SetIndexOfSplines _index)
    (if (Variables|Default|GetShowBulbs)
      (Components|InstancedStaticMesh|AddInstance (Variables|Default|GetInstancedBulb) (CallFunction|BulbPlacementCalculation) false)
      (if (Variables|LightningSettings|GetIsLightEnabled?)
        ;[1 1 1] Point Lights Settings
        (CallFunction|PointLightSetup (CallFunction|BulbPlacementCalculation))
        ;[1 1 1] Bulb settings setup
        (CallFunction|BulbSetup)
        (else
          (CallFunction|BulbSetup)
          (CallFunction|SplineMeshSetup)))
      (else
        ;[1 1 1] Spline and Wire Setup
        (CallFunction|SplineMeshSetup)))))

(fn GetLocationatIndex
  (params (A :type Integer))
  (return (Spline|GetLocationatDistanceAlongSpline (Variables|Default|GetSpline) (* A (Variables|Default|GetSpacing)) "Local")))

(fn BulbPlacementCalculation
  (bind _indexofsplines (Variables|Default|GetIndexOfSplines))
  (bind _returnvalue (CallFunction|GetLocationatIndex _indexofsplines))
  (bind _returnvalue_2 (+ _indexofsplines 1))
  (bind _returnvalue_3 (CallFunction|GetLocationatIndex _returnvalue_2))
  (bind _returnvalue_4 (- _returnvalue_3 _returnvalue))
  (bind _returnvalue_5 (Math|Rotator|MakeRotfromX _returnvalue_4))
  (bind (_roll _pitch _yaw) (Math|Rotator|BreakRotator _returnvalue_5))
  (return (Math|Transform|MakeTransform _returnvalue (Math|Rotator|MakeRotator 1.8e+02 _pitch _yaw))))

(fn PointLightSetup
  (params (InTransform :type Transform%20%28by%20ref%29))
  (bind (_location _rotation _scale) (Math|Transform|BreakTransform InTransform))
  (bind _returnvalue (AddComponent|AddPointLightComponent false (Math|Transform|MakeTransform (Math|Vector|MakeVector (.x _location) (.y _location) (- (.z _location) (Variables|LightningSettings|GetLight%20Position%20Offset))) _rotation _scale)))
  (Rendering|Components|Light|SetLightColor _returnvalue (Variables|LightningSettings|GetColor%20Value) true)
  (Rendering|Lighting|SetAttenuationRadius _returnvalue (Variables|LightningSettings|GetPointLightAttenuationRadius))
  (Rendering|Components|Light|SetIntensity _returnvalue (Variables|LightningSettings|GetPointLightIntensity)))

(fn BulbSetup
  (bind _returnvalue (Rendering|Material|CreateDynamicMaterialInstance (Variables|Default|GetInstancedBulb) 1 0 "None" :!class /Script/Engine.PrimitiveComponent))
  (Rendering|Material|SetVectorParameterValue _returnvalue "Emissive Color" (Variables|LightningSettings|GetColor%20Value) :!class /Script/Engine.MaterialInstanceDynamic)
  (Rendering|Material|SetScalarParameterValue _returnvalue "Emissive Strength" (Variables|LightningSettings|GetEmissive%20Strengh) :!class /Script/Engine.MaterialInstanceDynamic)
  (Rendering|Material|SetScalarParameterValue _returnvalue "Refraction Min" (Variables|LightningSettings|GetRefraction%20Min) :!class /Script/Engine.MaterialInstanceDynamic)
  (Rendering|Material|SetScalarParameterValue _returnvalue "Refraction Max" (Variables|LightningSettings|GetRefraction%20Max) :!class /Script/Engine.MaterialInstanceDynamic))

(fn SplineMeshSetup
  (bind _indexofsplines (Variables|Default|GetIndexOfSplines))
  (bind _indexofsplines_2 (Variables|Default|GetIndexOfSplines))
  (bind _fakegravitymin (Variables|Default|GetFakeGravityMin))
  (bind _fakegravitymax (Variables|Default|GetFakeGravityMax))
  (bind _spline (Variables|Default|GetSpline))
  (bind _spline_2 (Variables|Default|GetSpline))
  (bind _wiresectionlength (Variables|Default|GetWireSectionLength))
  (bind _wiresectionlength_2 (Variables|Default|GetWireSectionLength))
  (bind _returnvalue (* _wiresectionlength_2 _indexofsplines_2))
  (bind _returnvalue_2 (+ _indexofsplines 1))
  (bind _returnvalue_3 (* _wiresectionlength _returnvalue_2))
  (bind _returnvalue_4 (AddComponent|AddSplineMeshComponent false))
  (SplineMesh|SetForwardAxis _returnvalue_4 "Z" true)
  (Components|StaticMesh|SetStaticMesh _returnvalue_4 (Variables|Default|GetPlacesSplineMesh))
  (SplineMesh|SetStartandEnd _returnvalue_4 (Spline|GetLocationatDistanceAlongSpline _spline_2 _returnvalue "Local") (Math|Vector|ClampVectorSize (Spline|GetTangentatDistanceAlongSpline _spline_2 _returnvalue "Local") _fakegravitymin _fakegravitymax) (Spline|GetLocationatDistanceAlongSpline _spline _returnvalue_3 "Local") (Math|Vector|ClampVectorSize (Spline|GetTangentatDistanceAlongSpline _spline _returnvalue_3 "Local") _fakegravitymin _fakegravitymax) true :!class /Script/Engine.SplineMeshComponent))