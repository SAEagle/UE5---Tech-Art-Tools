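; Day/night cycle Blueprint that advances a game clock and drives the Sun and SkyLight from it.
; The construction script converts Day, Hour, Minute and Second to seconds, previewing lighting in the editor.
; A looping timer, its interval inversely scaled by Speed with a floor, drives time updates.
; Curves sampled by hour set sun pitch and skylight intensity and color; the per-tick time display is disconnected.
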(event EventBeginPlay
  (Utilities|Time|SetTimerbyEvent (EventDispatchers|CreateEvent :!event ChangeTime) (CallFunction|GetTimerRate) true))

(event EventTick
  (params (DeltaSeconds :type Float%20%28single-precision%29))
  (CallFunction|DisplayTime))

(fn ConstructionScript
  (Variables|Default|SetTime (Math|Conversions|ToFloat(Integer) (+ (* (Variables|Default|GetDay) 86400) (* (Variables|Default|GetHour) 3600) (* (Variables|Default|GetMinute) 60) (Variables|Default|GetSecond))))
  (CallFunction|UpdateAll))

(fn GetTimerRate
  (return (Math|Float|Max(Float) (/ 1e+01 (Variables|Default|GetSpeed)) 0.01)))

(fn ChangeTime
  (Variables|Default|SetTime (+ (Variables|Default|GetTime) (* (Variables|Default|GetSpeed) (CallFunction|GetTimerRate))))
  (CallFunction|UpdateAll))

(fn GetHour
  (return (/ (Math|Float|%(Float) (Variables|Default|GetTime) 8.64e+04) 3.6e+03)))

(fn GetDay
  (return (/ (Variables|Default|GetTime) 8.64e+04)))

(fn GetTimeSpan
  (return (Math|Timespan|MakeTimespan 0 0 0 (Math|Float|Truncate (Variables|Default|GetTime)))))

(fn DisplayTime
  (return))

(fn UpdateAll
  (CallFunction|UpdateSunDirection))

(fn UpdateSunDirection
  (bind _sun (Variables|Default|GetSun))
  (Utilities|IsValid _sun
    (:Is%20Valid
      (Transformation|SetActorRotation _sun (Math|Rotator|MakeRotator 0.0 (Math|Curves|GetFloatValue (Variables|Curve|GetCurveDirLight_X) (CallFunction|GetHour)) 0.0))
      (Rendering|Components|Light|SetIntensity (Variables|/Script/Engine.SkyLight|GetLightComponent (Variables|Default|GetSkyLight)) (Math|Curves|GetFloatValue (Variables|Curve|GetCurveSkyLightIntensity) (CallFunction|GetHour)))
      (Rendering|Components|Light|SetLightColor (Variables|/Script/Engine.SkyLight|GetLightComponent (Variables|Default|GetSkyLight)) (Math|Curves|GetLinearColorValue (Variables|Curve|GetCurveLinearColor) (CallFunction|GetHour)))
      (return))))